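; Asteroid actor for a space shooter that scores points when shot and triggers game over when it hits the player ship.
; The construction script randomizes spin, planar direction, mesh and material.
; Laser hits add score scaled by ScoreMultiplier and spawn two smaller copies with an incremented multiplier until it exceeds a limit, with a small collectible drop chance.
; Ship hits destroy both actors, spawn a larger explosion and show W_GameOver.
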(event `self.ReceiveActorBeginOverlap`
  (params (OtherActor :type "Actor Object Reference"))
  (bind _returnvalue (`GameplayStatics.GetPlayerController` 0))
  (bind _returnvalue_2 (`KismetMathLibrary.MakeTransform` (`self.deathLocation`) (struct) (* (.scale (`self.GetTransform`)) 0.75)))
  ;[1 1 1] Overlap with laser, increase score
  (bind _asbp_laser (cast `/Game/Blueprints/BP_Laser` OtherActor)
    (:`then`
      (`self.K2_DestroyActor` _asbp_laser)
      (set `self.deathLocation` (`SceneComponent.K2_GetComponentLocation` (`self.Asteroid`)))
      (bind _asbp_player_controller (cast `/Game/Blueprints/BP_PlayerController` _returnvalue))
      (set `/Game/Blueprints/BP_PlayerController.Score` (+ (* (`self.Score Multiplier`) 100) (`/Game/Blueprints/BP_PlayerController.Score` _asbp_player_controller)) _asbp_player_controller)
      (`/Engine/EditorBlueprintResources/StandardMacros.IncrementInt` (`/Game/Blueprints/BP_PlayerController.AsteroidsDestroyed` _asbp_player_controller)
        (:`  `
          (`GameplayStatics.PlaySound2D` "/Game/Sounds/S_explosion_asteroid.S_explosion_asteroid")
          (`|SpawnActorFromClass` "/Game/Blueprints/E_Explosion.E_Explosion_C" (`KismetMathLibrary.MakeTransform` (.location (`self.GetTransform`))) "Undefined" "OverrideRootScale" null null)
          ;[1 1 1] Spawn 2 asteroids with .75 scale
          (if (<= (`self.Score Multiplier`) 2)
            (bind _returnvalue_3 (`|SpawnActorFromClass` "BP_Asteroid_C" _returnvalue_2 "Undefined" "OverrideRootScale" null null))
            (set `/Game/Blueprints/BP_Asteroid.Score Multiplier` (+ (`self.Score Multiplier`) 1) _returnvalue_3)
            (bind _returnvalue_4 (`|SpawnActorFromClass` "BP_Asteroid_C" _returnvalue_2 "Undefined" "OverrideRootScale" null null))
            (set `/Game/Blueprints/BP_Asteroid.Score Multiplier` (+ (`self.Score Multiplier`) 1) _returnvalue_4)
            (`self.ChanceToSpawnCollectible`)
            (else
              (`self.ChanceToSpawnCollectible`))))))
    (:`CastFailed`
      ;[1 1 1] Overlap with ship, display game over screen
      (bind _asbp_player_ship_pawn (cast `/Game/Blueprints/BP_PlayerShipPawn` OtherActor))
      (`self.K2_DestroyActor` _asbp_player_ship_pawn)
      (`self.K2_DestroyActor`)
      (`GameplayStatics.PlaySound2D` "/Game/Sounds/S_explosion_player.S_explosion_player")
      (`|SpawnActorFromClass` "/Game/Blueprints/E_Explosion.E_Explosion_C" (`KismetMathLibrary.MakeTransform` (.location (`self.GetTransform`)) (struct) (5.0 5.0 5.0)) "Undefined" "OverrideRootScale" null null)
      (bind _returnvalue_5 (`|CreateWidget` "/Game/Blueprints/W_GameOver.W_GameOver_C" _returnvalue))
      (`UserWidget.AddToViewport` _returnvalue_5 0))))

(fn `ChanceToSpawnCollectible`
  ;[1 1 1] Chance to drop 'Collectible'
  (if (<= (`KismetMathLibrary.RandomInteger` 101) 10)
    (`|SpawnActorFromClass` "/Game/Blueprints/BP_Collectible.BP_Collectible_C" (`KismetMathLibrary.Conv_VectorToTransform` (`self.deathLocation`)) "Undefined" "OverrideRootScale" null null)
    (`self.K2_DestroyActor`)
    (else
      (`self.K2_DestroyActor`))))

(fn `SelectAsteroidMaterial`
  (bind _asteroid (`self.Asteroid`))
  (switch `int` (`KismetMathLibrary.RandomInteger` 3)
    (:`0`
      (`PrimitiveComponent.SetMaterial` _asteroid 0 "/Game/Materials/M_AsteroidBlack.M_AsteroidBlack"))
    (:`1`
      (`PrimitiveComponent.SetMaterial` _asteroid 0 "/Game/Materials/M_AsteroidBrown.M_AsteroidBrown"))
    (:`2`
      (`PrimitiveComponent.SetMaterial` _asteroid 0 "/Game/Materials/M_AsteroidGrey.M_AsteroidGrey"))))

(fn `SelectStaticMesh`
  (bind _asteroid (`self.Asteroid`))
  (switch `int` (`KismetMathLibrary.RandomInteger` 3)
    (:`0`
      (`StaticMeshComponent.SetStaticMesh` _asteroid "/Game/Assets/Asteroid_01.Asteroid_01"))
    (:`1`
      (`StaticMeshComponent.SetStaticMesh` _asteroid "/Game/Assets/Asteroid_04.Asteroid_04"))
    (:`2`
      (`StaticMeshComponent.SetStaticMesh` _asteroid "/Game/Assets/Asteroid_05.Asteroid_05"))))

(fn `UserConstructionScript`
  (bind _returnvalue (`KismetMathLibrary.MakeVector` (`KismetMathLibrary.RandomFloatInRange` -1.0 1.0) (`KismetMathLibrary.RandomFloatInRange` -1.0 1.0)))
  ;[1 1 1] Set random roll and velocity, Select one of three meshes and materials at random
  (set `RotatingMovementComponent.RotationRate` (`KismetMathLibrary.RandomRotator` false) (`self.RotatingMovement`))
  (set `MovementComponent.Velocity` _returnvalue (`self.ProjectileMovement`))
  (set `self.forwardVector` _returnvalue)
  (`self.SelectStaticMesh`)
  (`self.SelectAsteroidMaterial`))