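; BP_OutterWall is the outer boundary actor for an Asteroids-style game, handling projectile cleanup and screen wrapping.
; On actor begin overlap, it destroys lasers and moves asteroids or the player ship to a computed wrap location.
; GetWrappingLocation line-traces from the object's velocity vector, used as a world point, toward that vector negated and scaled, returning the hit location as the opposite-side position.
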(event `self.ReceiveActorBeginOverlap`
  (params (OtherActor :type "Actor Object Reference"))
  ;[1 1 1] Destroy projectile, respawn ship/asteroid on opposite side
  (bind _asbp_laser (cast `/Game/Blueprints/BP_Laser` OtherActor)
    (:`then`
      (`self.K2_DestroyActor` _asbp_laser))
    (:`CastFailed`
      (bind _asbp_asteroid (cast `/Game/Blueprints/BP_Asteroid` OtherActor)
        (:`then`
          (bind _newparam (`self.GetWrappingLocation` _asbp_asteroid))
          (`SceneComponent.K2_SetWorldLocation` (`Actor.RootComponent` _asbp_asteroid) _newparam false false))
        (:`CastFailed`
          (bind _asbp_player_ship_pawn (cast `/Game/Blueprints/BP_PlayerShipPawn` OtherActor))
          (bind _newparam_2 (`self.GetWrappingLocation` _asbp_player_ship_pawn))
          (`SceneComponent.K2_SetWorldLocation` (`/Game/Blueprints/BP_PlayerShipPawn.Ship` _asbp_player_ship_pawn) _newparam_2 false false))))))

(fn `GetWrappingLocation`
  (params (`Wrapping Object` :type "Actor Object Reference"))
  (returns (NewParam :type "Vector Structure"))
  (bind _returnvalue (`self.GetVelocity` `Wrapping Object`))
  (bind _outhit (`KismetSystemLibrary.LineTraceSingle` :`Start` _returnvalue :`End` (* (`KismetMathLibrary.NegateVector` _returnvalue) 500) :`TraceChannel` "TraceTypeQuery3" :`bIgnoreSelf` false))
  (return (`.Location` (`GameplayStatics.BreakHitResult` _outhit))))

(fn `UserConstructionScript`)