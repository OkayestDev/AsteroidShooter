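; BP_PlayerShipPawn is the player-controlled ship pawn, placed at a fixed height above the world origin on BeginPlay.
; The forward axis feeds the Arrow component's forward vector into FloatingPawnMovement to propel the ship.
; The rotation axis turns the Ship component's world yaw by a fixed step per input tick, without delta-time scaling.
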(event `self.ReceiveBeginPlay`
  ;[1 1 1] Spawn ship
  (`SceneComponent.K2_SetWorldLocation` (`self.Root`) (0.0 0.0 20.0) false false))

(event `InputAxis|ShipForwardMovement`
  (params (AxisValue :type "Float (single-precision)"))
  ;[1 1 1] Propel Ship Forward
  (`PawnMovementComponent.AddInputVector` (`self.FloatingPawnMovement`) (* (`SceneComponent.GetForwardVector` (`self.Arrow`)) AxisValue) false))

(event `InputAxis|ShipRotation`
  (params (AxisValue :type "Float (single-precision)"))
  (bind _ship (`self.Ship`))
  ;[1 1 1] Change Ships rotation
  (`SceneComponent.K2_SetWorldRotation` _ship (`KismetMathLibrary.MakeRotator` (.roll (`SceneComponent.K2_GetComponentRotation` _ship)) (.pitch (`SceneComponent.K2_GetComponentRotation` _ship)) (+ (.yaw (`SceneComponent.K2_GetComponentRotation` _ship)) (* AxisValue 3.0))) false false))

(fn `UserConstructionScript`)